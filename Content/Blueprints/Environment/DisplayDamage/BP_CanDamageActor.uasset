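; BP_CanDamageActor is a damageable actor that shows a damage display whenever its health changes and destroys itself on death.
; AnyDamage passes negated damage to the TDSHealth component, whose OnHealthChange event spawns a BP_DisplayDamageActor at the actor's location plus PointSpawnHealthNumber.
; The spawned actor receives damage and health with the shield flag off; the random XY offset is zeroed, so it has no scatter.
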(event `self.TDSHealth.OnDead`
  (`self.K2_DestroyActor`))

(event `self.TDSHealth.OnHealthChange`
  (params (Health :type "Float (single-precision)") (Damage :type "Float (single-precision)"))
  ;[0.5608 0 0.7333] Спавнем актора, в котором компонент виджета и
  (bind _returnvalue (`|SpawnActorFromClass` "/Game/Blueprints/Environment/DisplayDamage/BP_DisplayDamageActor.BP_DisplayDamageActor_C" (`KismetMathLibrary.MakeTransform` (+ (+ (`KismetMathLibrary.MakeVector` (`KismetMathLibrary.RandomFloatInRange` 0.0) (`KismetMathLibrary.RandomFloatInRange` 0.0)) (`self.PointSpawnHealthNumber`)) (`self.K2_GetActorLocation`))) "Undefined" "OverrideRootScale" null null))
  (`/Game/Blueprints/Environment/DisplayDamage/BP_DisplayDamageActor.InitActorEvent` _returnvalue Damage Health false))

(event `self.ReceiveAnyDamage`
  (params (Damage :type "Float (single-precision)") (DamageType :type "DamageType Object Reference") (InstigatedBy :type "Controller Object Reference") (DamageCauser :type "Actor Object Reference"))
  (`TDSHealthComponent.ChangeHealthValue` (`self.TDSHealth`) (* Damage -1.0)))

(fn `UserConstructionScript`)