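; Weapon pickup actor that hands its weapon to an overlapping character's inventory.
; On BeginPlay it looks up drop info by item name in BP_GameInstance, and InitActor uses the info to set a static or skeletal mesh and particle effect.
; If the inventory rejects the weapon, it starts a weapon-switch on BP_Character, which ends when the character leaves the sphere.
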(event `self.ReceiveBeginPlay`
  (bind _itemname (`self.ItemName`))
  (`parent.ReceiveBeginPlay`)
  (if (!= _itemname "None")
    (bind _asbp_game_instance (cast `/Game/Blueprints/GameInstance/BP_GameInstance` (`GameplayStatics.GetGameInstance`)))
    (bind (_outinfo _returnvalue) (`TDSGameInstance.GetDropItemInfoByName` _asbp_game_instance _itemname))
    (if _returnvalue
      (set `self.Weapon Info` _outinfo)))
  (`self.InitActor` (`self.Weapon Info`)))

(event `self.OverlapCharacter`
  (params (ToInventory :type "TDSInventoryComponent Object Reference"))
  (`parent.OverlapCharacter` ToInventory)
  (bind _returnvalue (`TDSInventoryComponent.TryGetWeaponToInventory` ToInventory (`.WeaponInfo` (break `DropItem` (`self.Weapon Info`)))))
  (if _returnvalue
    (`self.PickUpSuccess`)
    (else
      (bind _asbp_character (cast `/Game/Blueprints/Character/BP_Character` (`ActorComponent.GetOwner` ToInventory)))
      (`/Game/Blueprints/Character/BP_Character.StartSwitchWeapon` _asbp_character self))))

(event `self.Sphere.OnComponentEndOverlap`
  (params (OverlappedComponent :type "PrimitiveComponent Object Reference") (OtherActor :type "Actor Object Reference") (OtherComp :type "PrimitiveComponent Object Reference") (OtherBodyIndex :type Integer))
  (bind _asbp_character (cast `/Game/Blueprints/Character/BP_Character` OtherActor))
  (`/Game/Blueprints/Character/BP_Character.EndSwitchWeapon` _asbp_character))

(fn `InitActor`
  (params (InfoActor :type "DropItem Structure"))
  (bind (_weaponstaticmesh _weaponskeletmesh _weaponinfo) (break `DropItem` InfoActor))
  (bind _weaponstaticmesh_2 (`self.WeaponStaticMesh`))
  (bind _weaponskeletalmesh (`self.WeaponSkeletalMesh`))
  (bind _particlesystem (`self.ParticleSystem`))
  (`|ExecutionSequence`
    (:`then_0`
      (`/Engine/EditorBlueprintResources/StandardMacros.IsValid` _weaponstaticmesh
        (:`Is Valid`
          (`ActorComponent.K2_DestroyComponent` (`self.WeaponStaticMesh`))
          (`StaticMeshComponent.SetStaticMesh` _weaponstaticmesh_2 _weaponstaticmesh)
          (`SceneComponent.K2_SetRelativeLocation` _weaponstaticmesh_2 (0.0 0.0 0.0) false false))
        (:`Is Not Valid`
          (`/Engine/EditorBlueprintResources/StandardMacros.IsValid` _weaponskeletmesh
            (:`Is Valid`
              (`ActorComponent.K2_DestroyComponent` (`self.WeaponStaticMesh`))
              (`SkinnedMeshComponent.SetSkinnedAssetAndUpdate` _weaponskeletalmesh _weaponskeletmesh true)
              (`SceneComponent.K2_SetRelativeLocation` _weaponskeletalmesh (0.0 0.0 0.0) false false))
            (:`Is Not Valid`
              (`KismetSystemLibrary.PrintString` "Error Drop Item Not have any MESH" true true (struct :`R` 1.0 :`G` 0.061242 :`A` 1.0)))))))
    (:`then_1`
      (`/Engine/EditorBlueprintResources/StandardMacros.IsValid` null
        (:`Is Valid`
          (`ParticleSystemComponent.SetTemplate` _particlesystem null)
          (`SceneComponent.SetRelativeScale3D` _particlesystem (0.3 0.3 0.3)))
        (:`Is Not Valid`
          (`ActorComponent.K2_DestroyComponent` _particlesystem))))
    (:`then_2`
      (set `self.ItemName` (`.NameItem` (break `WeaponSlot` _weaponinfo))))))

(fn `UserConstructionScript`
  (`parent.UserConstructionScript`))