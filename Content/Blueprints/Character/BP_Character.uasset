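; Top-down character Blueprint handling camera setup, weapon reload animation and weapon-switch UI.
; Construction configures the boom's height, angle and lag; F triggers a camera shake, and Tick prints weapon debug state.
; Reload events forward to ABP_MannyMain, while switch events show or remove the SwitchWeapon widget and track the pickup.
; Numbered slot-swap logic, which drops the replaced weapon as a pickup, has no connected trigger; CameraSlide is uncalled here.
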(event `self.ReceiveTick`
  (params (DeltaSeconds :type "Float (single-precision)"))
  (bind _returnvalue (`self.GetCurrentWeapon`))
  (`/Engine/EditorBlueprintResources/StandardMacros.IsValid` _returnvalue
    (:`Is Valid`
      (bind _returnvalue_2 (`WeaponDefault.GetWeaponRound` _returnvalue))
      (`KismetSystemLibrary.PrintString` (`KismetStringLibrary.Concat_StrStr` "IsFiring = " (`KismetStringLibrary.Conv_BoolToString` (`WeaponDefault.WeaponFiring` _returnvalue)) "|| isReloading = " (`KismetStringLibrary.Conv_BoolToString` (`WeaponDefault.WeaponReloading` _returnvalue)) "||| CurrentRound = " (`KismetStringLibrary.Conv_IntToString` _returnvalue_2)) true true (struct :`A` 1.0) 0.0))))

(event `self.WeaponReloadStart_BP`
  (params (Anim :type "AnimMontage Object Reference"))
  (`/Game/Blueprints/Character/Characters/Mannequins/Animations/ABP_MannyMain.Reload` (`self.Character Anim Instance`) Anim))

(event `self.WeaponReloadEnd_BP`
  (params (bIsSuccess :type Boolean))
  (`/Game/Blueprints/Character/Characters/Mannequins/Animations/ABP_MannyMain.Reload` (`self.Character Anim Instance`) null))

(event `self.ReceiveBeginPlay`
  (bind _asabp_manny_main (cast `/Game/Blueprints/Character/Characters/Mannequins/Animations/ABP_MannyMain` (`SkeletalMeshComponent.GetAnimInstance` (`self.Mesh`))))
  (set `self.Character Anim Instance` _asabp_manny_main))

(event `Key|F`
  (params (Key :type "Key Structure"))
  (:`Pressed`
    (`self.CameraShakeEvent`)))

(event `StartSwitchWeapon`
  (params (CatchPickUpWeapon :type "/Game/Blueprints/InteractionEnvironment/PickUpActor_Weapon Object Reference"))
  (bind _returnvalue (`|CreateWidget` "/Game/Blueprints/Widgets/Inventory/SwitchWeapon.SwitchWeapon_C"))
  (bind _output_get (set `self.SwitchWeaponWidget` _returnvalue))
  (`UserWidget.AddToViewport` _output_get 0)
  (set `self.CatchPickUpWeapon` CatchPickUpWeapon))

(event `EndSwitchWeapon`
  (bind _switchweaponwidget (`self.SwitchWeaponWidget`)
    (:`then`
      (`Widget.RemoveFromParent` _switchweaponwidget))
    (:`else`
      _))
  (set `self.SwitchWeaponWidget` null)
  (set `self.CatchPickUpWeapon` null))

(event `InputAction|ActionNum1`
  (params (Key :type "Key Structure")))

(event `InputAction|ActionNum2`
  (params (Key :type "Key Structure")))

(event `InputAction|ActionNum3`
  (params (Key :type "Key Structure")))

(event `InputAction|ActionNum4`
  (params (Key :type "Key Structure")))

(fn `Camera Slide`
  (params (Value :type "Float (double-precision)"))
  (returns (NewCameraHeight :type "Float (double-precision)") (ReturnValue :type "Float (double-precision)"))
  (bind _cameraboom (`self.CameraBoom`))
  (bind (_returnvalue_roll _returnvalue_pitch) (`KismetMathLibrary.BreakRotator` (`SceneComponent.K2_GetComponentRotation` _cameraboom)))
  (bind _returnvalue (* Value (`self.HeightCameraChangeDistance`)))
  (return (+ _returnvalue (`SpringArmComponent.TargetArmLength` _cameraboom)) (+ _returnvalue_pitch (* (/ _returnvalue 100.0) -1.0))))

(fn `CameraShakeEvent`
  (`GameplayStatics.PlayWorldCameraShake` "/Game/Blueprints/Environment/BP_ShakeCamera.BP_ShakeCamera_C" (`SceneComponent.K2_GetComponentLocation` (`self.TopDownCameraComponent`)) 0.0 10.0))

(fn `Drop Item`
  (params (DropItemInfo :type "DropItem Structure"))
  (`|SpawnActorFromClass` "/Game/Blueprints/InteractionEnvironment/PickUpActor_Weapon.PickUpActor_Weapon_C" (`KismetMathLibrary.MakeTransform` (+ (`self.K2_GetActorLocation`) (* (`self.GetActorForwardVector`) 1.0))) "AdjustIfPossibleButAlwaysSpawn" "OverrideRootScale" null DropItemInfo null))

(fn `UserConstructionScript`
  (bind _cameraboom (`self.CameraBoom`))
  (set `SpringArmComponent.TargetArmLength` (`self.HeightCameraMax`) _cameraboom)
  (`SceneComponent.K2_SetRelativeRotation` _cameraboom (`self.RotatorCamera`) false false)
  (set `SpringArmComponent.bEnableCameraLag` (`self.Flow`) _cameraboom)
  (set `SpringArmComponent.CameraLagSpeed` (`self.CoefSmooth`) _cameraboom))