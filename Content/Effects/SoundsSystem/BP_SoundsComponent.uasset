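; Actor component that plays footstep, landing, phrase and main sounds at its owner.
; Step and fall functions trace downward, pick a sound by physical surface type and play it at the hit location.
; The FPS step variant accumulates delta time while the owner moves to space out footsteps.
; Phrase and main functions accept override sounds; the music event only plays when not looping, as looping is unfinished.
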(event `PlayMusicEvent`
  (params (Sounds_Main :type "SoundBase Object Reference") (Loop :type Boolean))
  ;[1 1 1] Лупит поданный трек или играет саундмаин
  (`/Engine/EditorBlueprintResources/StandardMacros.IsValid` Sounds_Main
    (:`Is Valid`
      (set `self.Sounds_Main` Sounds_Main))
    (:`Is Not Valid`
      _))
  (bind _output_get (set `self.Loop` Loop))
  (if (not _output_get)
    (`GameplayStatics.PlaySoundAtLocation` (`self.Sounds_Main`) (`Actor.K2_GetActorLocation` (`self.GetOwner`)) (struct) 1.0 1.0 0.0 null null null)))

(fn `fPlaySound_Falls`
  (bind _returnvalue (`self.GetOwner`))
  (bind _sound_fall_beton (`self.Sound_Fall_Beton`))
  (bind _returnvalue_2 (`Actor.K2_GetActorLocation` _returnvalue))
  (bind _outhit (`KismetSystemLibrary.LineTraceSingle` _returnvalue_2 (- _returnvalue_2 (0.0 0.0 200.0)) "TraceTypeQuery1" false (`|MakeArray` _returnvalue)))
  (`GameplayStatics.PlaySoundAtLocation` (select `EPhysicalSurface` (`GameplayStatics.GetSurfaceType` _outhit) :`SurfaceType_Default` _sound_fall_beton :`SurfaceType1` _sound_fall_beton :`SurfaceType2` (`self.Sound_Fall_Wood`) :`SurfaceType3` (`self.Sound_Fall_Metal`) :`SurfaceType4` (`self.Sound_Steps_Water`)) (`.Location` (`GameplayStatics.BreakHitResult` _outhit)) (struct) 1.0 1.0 0.0 null null null)
  (return))

(fn `fPlaySound_Main`
  (params (SetNewSound :type "SoundBase Object Reference") (StartTime :type "Float (double-precision)"))
  (`/Engine/EditorBlueprintResources/StandardMacros.IsValid` SetNewSound
    (:`Is Valid`
      (bind _output_get (set `self.Sounds_Main` SetNewSound)))
    (:`Is Not Valid`
      _))
  (`GameplayStatics.PlaySoundAtLocation` _output_get (`Actor.K2_GetActorLocation` (`self.GetOwner`)) (struct) 1.0 1.0 StartTime null null null)
  (return))

(fn `fPlaySound_Phrase`
  (params (Sound :type "SoundBase Object Reference"))
  (bind _returnvalue (`Actor.K2_GetActorLocation` (`self.GetOwner`)))
  (`/Engine/EditorBlueprintResources/StandardMacros.IsValid` Sound
    (:`Is Valid`
      (`GameplayStatics.PlaySoundAtLocation` Sound _returnvalue (struct) 1.0 1.0 0.0 null null null))
    (:`Is Not Valid`
      (`GameplayStatics.PlaySoundAtLocation` (`self.Sounds_Phrase`) _returnvalue (struct) 1.0 1.0 0.0 null null null))))

(fn `fPlaySound_Steps`
  (bind _returnvalue (`self.GetOwner`))
  (bind _returnvalue_2 (`Actor.K2_GetActorLocation` _returnvalue))
  (bind _outhit (`KismetSystemLibrary.LineTraceSingle` _returnvalue_2 (- _returnvalue_2 (0.0 0.0 200.0)) "TraceTypeQuery1" false (`|MakeArray` _returnvalue)))
  (`GameplayStatics.PlaySoundAtLocation` (select `EPhysicalSurface` (`GameplayStatics.GetSurfaceType` _outhit) :`SurfaceType_Default` (`self.Sound_Steps_Default`) :`SurfaceType1` (`self.Sound_Steps_Beton`) :`SurfaceType2` (`self.Sound_Steps_Wood`) :`SurfaceType3` (`self.Sound_Steps_Metal`) :`SurfaceType4` (`self.Sound_Steps_Water`) :`SurfaceType5` (`self.Sound_Steps_Bone`)) (`.Location` (`GameplayStatics.BreakHitResult` _outhit)) (struct) 1.0 1.0 0.0 null null null)
  (return))

(fn `fPlaySound_StepsFPS`
  (bind _returnvalue (`self.GetOwner`))
  (bind _sound_steps_beton (`self.Sound_Steps_Beton`))
  (bind _returnvalue_2 (`Actor.K2_GetActorLocation` _returnvalue))
  (if (> (`KismetMathLibrary.VSize` (`Actor.GetVelocity` (`self.GetOwner`))) 0.0)
    (set `self.Count` (+ (`self.Count`) (`GameplayStatics.GetWorldDeltaSeconds`)))
    (if (> (`self.Count`) 0.35)
      (bind _outhit (`KismetSystemLibrary.LineTraceSingle` _returnvalue_2 (- _returnvalue_2 (0.0 0.0 200.0)) "TraceTypeQuery1" false (`|MakeArray` _returnvalue)))
      (`GameplayStatics.PlaySoundAtLocation` (select `EPhysicalSurface` (`GameplayStatics.GetSurfaceType` _outhit) :`SurfaceType_Default` _sound_steps_beton :`SurfaceType1` _sound_steps_beton :`SurfaceType2` (`self.Sound_Steps_Wood`) :`SurfaceType3` (`self.Sound_Steps_Metal`) :`SurfaceType4` (`self.Sound_Steps_Water`)) (`.Location` (`GameplayStatics.BreakHitResult` _outhit)) (struct) 1.0 1.0 0.0 null null null)
      (set `self.Count` 0.0))
    (else
      (set `self.Count` 0.0))))

(fn `fPlaySound_TEST`
  (params (Play :type Boolean))
  (returns (Sounds_Main :type "SoundBase Object Reference"))
  (bind _sounds_main (`self.Sounds_Main`))
  ;[1 1 1] Тестовый функционал
  (if Play
    (`GameplayStatics.PlaySoundAtLocation` _sounds_main (`Actor.K2_GetActorLocation` (`self.GetOwner`)) (struct) 1.0 1.0 0.0 null null null)
    ;[1 1 1] добавь время прошедшее с начала
    (return _sounds_main)))